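; BP_test_Sphere is a test sphere actor that opens a material selection UI when an actor overlaps it.
; On overlap it creates BP_Widget_interface and fills HorizontalBox3 with a numbered WBP_Button per Materials entry, built by the NewMacro macro to target SphereMesh.
; It shows the cursor with game-and-UI input; EndInteract removes the widgets and restores game-only input.
; Click, component overlap and overlay-material handlers are empty stubs.
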(event `self.ReceiveBeginPlay`)

(event `self.SphereMesh.OnClicked`
  (params (TouchedComponent :type "PrimitiveComponent Object Reference") (ButtonPressed :type "Key Structure")))

(event `Set OverlayMat`
  (params (`OverlayMat Bool` :type Boolean))
  (if (`self.Overlay Mat Bool`)
    _))

(event `self.ReceiveActorBeginOverlap`
  (params (OtherActor :type "Actor Object Reference"))
  (bind _returnvalue (`GameplayStatics.GetPlayerController` 0))
  (bind _returnvalue_2 (`GameplayStatics.GetPlayerController` 0))
  ;[0.6922 0.5444 1] Material
  (bind _returnvalue_3 (`|CreateWidget` "/Game/Blueprint/BP_Essai_1/BP_Widget_interface.BP_Widget_interface_C" _returnvalue))
  (`UserWidget.AddToViewport` _returnvalue_3 0)
  (for (_array_element _array_index) (`self.Materials`)
    (bind _outputpin (`self.NewMacro` _array_element _returnvalue (`KismetStringLibrary.Conv_IntToString` (+ _array_index 1))))
    (`PanelWidget.AddChild` (`/Game/Blueprint/BP_Essai_1/BP_Widget_interface.HorizontalBox_3` _returnvalue_3) _outputpin)
    (`UserWidget.AddToViewport` _returnvalue_3 0)
    (`WidgetBlueprintLibrary.SetInputMode_GameAndUIEx` _returnvalue_2 _returnvalue_3 "DoNotLock" false)
    (set `PlayerController.bShowMouseCursor` true _returnvalue_2)))

(event `self.SphereMesh.OnComponentBeginOverlap`
  (params (OverlappedComponent :type "PrimitiveComponent Object Reference") (OtherActor :type "Actor Object Reference") (OtherComp :type "PrimitiveComponent Object Reference") (OtherBodyIndex :type Integer) (bFromSweep :type Boolean) (SweepResult :type "HitResult Structure (by ref)")))

(event `EndInteract`
  (bind _returnvalue (`GameplayStatics.GetPlayerController` 0))
  ;[0.6922 0.5444 1] Material
  (`/Engine/EditorBlueprintResources/StandardMacros.IsValid` null
    (:`Is Valid`
      (`Widget.RemoveFromParent` (stale `self.ReceiveActorBeginOverlap` _returnvalue_3)))
    (:`Is Not Valid`
      _))
  (`Widget.RemoveFromParent` (`self.widget E`))
  (`WidgetBlueprintLibrary.SetInputMode_GameOnly` _returnvalue) ; set back input game mode
  (set `PlayerController.bShowMouseCursor` false _returnvalue)
  (set `self.Interact    Bool` false))

(fn `UserConstructionScript`)