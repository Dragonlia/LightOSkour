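; BP_Interaction is a first-person interactable that acts as a light switch, a door or a mesh material picker.
; HitInteractBP follows the character's hit state to toggle the overlay highlight and "Press E" prompt, opening or closing a Gate that IA_PressE enters.
; E flip-flops light visibility, swings the door via timeline, or toggles a three-color choice widget with cursor input.
; SetMatLoop applies the chosen material across StaticMeshList's mesh/slot pairs.
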(event `Set Mat loop`
  (params (Index :type Integer))
  (bind _staticmeshlist (`self.StaticMeshList`))
  ;[1 0.3534 0.3833 1 50] Set materials Loops
  (bind _keys (`BlueprintMapLibrary.Map_Keys` _staticmeshlist))
  (bind _values (`BlueprintMapLibrary.Map_Values` _staticmeshlist))
  (for (_array_element _array_index) _keys
    (`PrimitiveComponent.SetMaterial` (`StaticMeshActor.StaticMeshComponent` (`|ConvertAsset` _array_element)) (`|GetArrayItem` _values _array_index) (select `int` Index :`0` (`self.Material0`) :`1` (`self.Material1`) :`2` (`self.Material2`)))))

(event `EnhancedInput|/Game/Blueprint/Input/IA_PressE`
  (params (ActionValue :type Boolean) (ElapsedSeconds :type "Float (double-precision)") (TriggeredSeconds :type "Float (double-precision)") (InputAction :type "InputAction Object Reference" :default "/Game/Blueprint/Input/IA_PressE.IA_PressE"))
  (bind _rootcomponent (`Actor.RootComponent` (`|ConvertAsset` (`self.Light Switch`))))
  ;[0.2146 0.08658 0.5729 1 50] Enter/Exit interaction mode
  ;;[1 1 1] Input E
  (:`Started`
    ;;[1 1 1] Gate interaction: enter/exit
    (`/Engine/EditorBlueprintResources/StandardMacros.Gate` true :!label _label
      (:`Exit`
        (if (`self.Light?`)
          (`/Engine/EditorBlueprintResources/StandardMacros.FlipFlop`
            (:`A`
              (`SceneComponent.SetVisibility` _rootcomponent false false))
            (:`B`
              (`SceneComponent.SetVisibility` _rootcomponent true false)))
          (elif (`self.Door?`)
            ;;[1 1 1] Door Interaction
            (`/Game/Blueprint/Interact/BP_Door.OpenDoor` (`|ConvertAsset` (`self.BP_door`)))
            (`/Engine/EditorBlueprintResources/StandardMacros.FlipFlop`
              (:`A`
                (bind (_direction _doortimeline) (`Timeline|Timeline` :!label _label_2)
                  (:`Update`
                    (`SceneComponent.K2_SetRelativeRotation` (`self.DefaultSceneRoot`) (`KismetMathLibrary.MakeRotator` 0.0 0.0 (* _doortimeline 90.0)) false false))))
              (:`B`
                (goto _label_2 :!via `Reverse`)))
            (elif (`self.InteractBool`)
              (bind _focusedbp (`/Game/FirstPerson/Blueprints/BP_FirstPersonCharacter.FocusedBP` (stale `HitInteractBP` _asbp_first_person_character)))
              (`self.Set Mat loop` _focusedbp (`self.Previous_Index`))
              (`self.EndInteract` _focusedbp) ; cancel interaction by pressing E
              (`self.Set OverlayMat` _focusedbp false)
              (else
                (`self.StartInteract` _focusedbp)
                (`self.Set OverlayMat` _focusedbp false)))))))))

(event `HitInteractBP`
  ;[0.2146 0.08658 0.5729 1 50] Enter/Exit interaction mode
  ;;[1 1 1] Cast from FPbp
  (bind _asbp_first_person_character (cast `/Game/FirstPerson/Blueprints/BP_FirstPersonCharacter` (`GameplayStatics.GetPlayerPawn` 0)))
  (if (`/Game/FirstPerson/Blueprints/BP_FirstPersonCharacter.HitBP` _asbp_first_person_character)
    (bind _focusedbp (`/Game/FirstPerson/Blueprints/BP_FirstPersonCharacter.FocusedBP` _asbp_first_person_character))
    (`self.EnableInput` _focusedbp (`GameplayStatics.GetPlayerController` 0))
    (`self.Set OverlayMat` _focusedbp true)
    ;;[1 1 1] Widget Interact - Press E
    (bind _returnvalue (`|CreateWidget` "/Game/Blueprint/UI/WBP_WIdget_PressE.WBP_WIdget_PressE_C"))
    (bind _output_get (set `self.Widget_PressE` _returnvalue))
    (`/Game/Blueprint/UI/WBP_WIdget_PressE.UpdateObjectText` _output_get (`self.Object Text`))
    (`UserWidget.AddToViewport` _output_get 0)
    (goto _label :!via `Open`)
    (else
      (`self.Set Mat loop` _focusedbp (`self.Previous_Index`))
      (`self.EndInteract` _focusedbp) ; Cancel interact by walking out
      (`self.Set OverlayMat` _focusedbp false)
      (goto _label :!via `Close`))))

(event `Set OverlayMat`
  (params (`OverlayMat Bool` :type Boolean))
  ;[1 0.3534 0.3833 1 50] Set materials Loops
  (if (`self.OverlayMat ?`)
    (bind _keys (`BlueprintMapLibrary.Map_Keys` (`self.StaticMeshList`)))
    (for _array_element _keys
      (if `OverlayMat Bool`
        (bind _staticmeshcomponent (`StaticMeshActor.StaticMeshComponent` (`|ConvertAsset` _array_element)))
        (`MeshComponent.SetOverlayMaterial` _staticmeshcomponent "/Game/Art/Overlays/MI_Overlay.MI_Overlay")
        (else
          (`MeshComponent.SetOverlayMaterial` _staticmeshcomponent null))))))

(event `Close Interaction Door`
  ;[0.2146 0.08658 0.5729 1 50] Enter/Exit interaction mode
  (goto _label :!via `Close`))

(event `StartInteract`
  (bind _returnvalue (`GameplayStatics.GetPlayerController` 0))
  ;[0 0.3718 1 1 50] Start/End Interaction
  (set `self.InteractBool` true)
  ;;[1 1 1] Add choice widget
  (bind _returnvalue_2 (`|CreateWidget` "/Game/Blueprint/UI/WBP_WidgetInteractable.WBP_WidgetInteractable_C"))
  (set `/Game/Blueprint/UI/WBP_WidgetInteractable.BP_interact` self _returnvalue_2)
  (`/Game/Blueprint/UI/WBP_WidgetInteractable.SetButtonsColors` _returnvalue_2 (`self.Color0`) (`self.Color1`) (`self.Color2`))
  (`UserWidget.AddToViewport` _returnvalue_2 0)
  ;;[1 1 1] Input interaction mode
  (`WidgetBlueprintLibrary.SetInputMode_GameAndUIEx` _returnvalue _returnvalue_2 "DoNotLock" false)
  (set `PlayerController.bShowMouseCursor` true _returnvalue))

(event `EndInteract`
  (bind _returnvalue (`GameplayStatics.GetPlayerController` 0))
  ;[0 0.3718 1 1 50] Start/End Interaction
  ;;[0.01042 0.01042 0.01042] End Interaction
  (`/Engine/EditorBlueprintResources/StandardMacros.IsValid` (stale `StartInteract` _returnvalue_2)
    (:`Is Valid`
      (`Widget.RemoveFromParent` (stale `StartInteract` _returnvalue_2)))
    (:`Is Not Valid`
      _))
  (`Widget.RemoveFromParent` (`self.Widget_PressE`))
  (`WidgetBlueprintLibrary.SetInputMode_GameOnly` _returnvalue) ; set back input game mode
  (set `PlayerController.bShowMouseCursor` false _returnvalue)
  (set `self.InteractBool` false))

(fn `UserConstructionScript`)